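; BP_WeaponBase is a base weapon Blueprint that handles magazine ammo, firing and timed reloads.
; FireWeapon spends a round, spawns muzzle particles and sound at the Arrow, then calls WeaponTrace, an empty event that child weapons can override.
; An empty magazine or Reload call enters a shared DoOnce that shows a WB_ReloadBar widget, waits ReloadTime, refills ammo and resets.
; It also exposes an FOV multiplier getter.
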(event `self.ReceiveBeginPlay`
  (set `self.Ammo` (`self.MaxMagazineAmmo`)))

(event `/Game/Blueprints/FirstPersonTemplate/BPL_Weapon.FireWeapon`
  (`/Engine/EditorBlueprintResources/StandardMacros.CompareInt` (`self.Ammo`)
    (:`>`
      (set `self.Ammo` (- (`self.Ammo`) 1))
      (`self.WeaponFireEffects`)
      (`self.WeaponTrace`))
    (:`==`
      (`self.ReloadWeapon` :!label _label))
    (:`<`
      (goto _label))))

(event `WeaponTrace`)

(event `ReloadWeapon`
  (`/Engine/EditorBlueprintResources/StandardMacros.DoOnce` false :!label _label_2
    (:`Completed`
      (bind _returnvalue (`|CreateWidget` "/Game/Blueprints/Weapons/WB_ReloadBar.WB_ReloadBar_C"))
      (`/Game/Blueprints/Weapons/WB_ReloadBar.ReloadAnimation` _returnvalue (`self.ReloadTime`))
      (`UserWidget.AddToViewport` _returnvalue 0)
      (`KismetSystemLibrary.Delay` (`self.ReloadTime`))
      (set `self.Ammo` (`self.MaxMagazineAmmo`))
      (goto _label_2 :!via `Reset`))))

(event `/Game/Blueprints/FirstPersonTemplate/BPL_Weapon.Reload`
  (goto _label_2))

(fn `GetFOVMultiplier`
  (returns (FOVMultiplier :type "Float (double-precision)"))
  (return (`self.FOVMultiplier`)))

(fn `UserConstructionScript`)

(fn `WeaponFireEffects`
  (bind (_returnvalue_location _returnvalue_rotation) (`KismetMathLibrary.BreakTransform` (`SceneComponent.K2_GetComponentToWorld` (`self.Arrow`))))
  (`GameplayStatics.SpawnEmitterAtLocation` (`self.WeaponFireEmitter`) _returnvalue_location _returnvalue_rotation (`self.WeaponFireEmitterScale`))
  (`GameplayStatics.SpawnSoundAtLocation` (`self.WeaponFireSound`) _returnvalue_location (struct) 1.0 1.0 0.0 null null)
  (return))